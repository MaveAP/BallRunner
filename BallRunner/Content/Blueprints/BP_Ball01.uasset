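; BP_Ball01 is a player-controlled ball that rolls by torque and jumps on SpaceBar.
; Both movement axes feed one AddTorqueInRadians node on the Sphere, which applies the axis value times StrMultiply to X and Y alike as an acceleration change.
; SpaceBar applies an upward velocity-change impulse if CanJump is true, then leaves the flag true, so this graph never blocks repeated jumps.
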(event Input|AxisEvents|InputAxisMoveForwardBack
  (params (AxisValue :type Float%20%28single-precision%29))
  (bind _str_multiply (Variables|BallPropertys|GetStr%20multiply))
  (Class|PrimitiveComponent|AddTorqueinRadians (Variables|Default|GetSphere) (Math|Vector|MakeVector (* (stale Input|AxisEvents|InputAxisMoveLeftRight AxisValue) _str_multiply) (* AxisValue _str_multiply) 0.0) "None" true))

(event Input|AxisEvents|InputAxisMoveLeftRight
  (params (AxisValue :type Float%20%28single-precision%29))
  (bind _str_multiply (Variables|BallPropertys|GetStr%20multiply))
  (Class|PrimitiveComponent|AddTorqueinRadians (Variables|Default|GetSphere) (Math|Vector|MakeVector (* AxisValue _str_multiply) (* (stale Input|AxisEvents|InputAxisMoveForwardBack AxisValue) _str_multiply) 0.0) "None" true))

(event Input|KeyboardEvents|SpaceBar
  (params (Key :type Key%20Structure :default "None"))
  (:Pressed
    (if (Variables|Default|GetCanJump)
      (Variables|Default|SetCanJump true)
      (Physics|AddImpulse (Variables|Default|GetSphere) "0, 0,500.000000" "None" true))))

(fn ConstructionScript)