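; A platform that tilts while the player's ball (BP_Ball01) is on it and levels out once the ball leaves.
; Box overlap events check for the player pawn, then set the tilt flag, target angle and interpolation speed.
; Tick eases the Cube's relative roll toward that angle or back to zero with FInterpTo on scaled-down delta time, holding pitch and yaw at zero.
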(event OnComponentBeginOverlap(Box)
  (params (OverlappedComponent :type Primitive%20Component%20Object%20Reference) (OtherActor :type Actor%20Object%20Reference) (OtherComp :type Primitive%20Component%20Object%20Reference) (OtherBodyIndex :type Integer) (bFromSweep :type Boolean) (SweepResult :type Hit%20Result%20Structure%20%28by%20ref%29))
  (bind _asbp_ball_01 (Utilities|Casting|CastToBP_Ball01 (Game|Player|GetPlayerPawn 0)))
  (if (== _asbp_ball_01 OtherActor)
    (Variables|MyBleprint|SetIsTilting true)
    (Variables|MyBleprint|SetTiltAngle 15.0)
    (Variables|MyBleprint|SetTiltSpeed 1e+01)))

(event OnComponentEndOverlap(Box)
  (params (OverlappedComponent :type Primitive%20Component%20Object%20Reference) (OtherActor :type Actor%20Object%20Reference) (OtherComp :type Primitive%20Component%20Object%20Reference) (OtherBodyIndex :type Integer))
  (bind _asbp_ball_01 (Utilities|Casting|CastToBP_Ball01 (Game|Player|GetPlayerPawn 0)))
  (if (== _asbp_ball_01 OtherActor)
    (Variables|MyBleprint|SetIsTilting false)
    (Variables|MyBleprint|SetTiltAngle 0.0)
    (Variables|MyBleprint|SetTiltSpeed 2e+01)))

(event EventTick
  (params (DeltaSeconds :type Float%20%28single-precision%29))
  (bind _returnvalue (* DeltaSeconds 0.1))
  (bind _cube (Variables|Default|GetCube))
  (bind _tiltspeed (Variables|MyBleprint|GetTiltSpeed))
  (bind _relativerotation (Variables|/Script/Engine.SceneComponent|GetRelativeRotation _cube))
  (bind _roll (Math|Rotator|BreakRotator _relativerotation))
  (if (Variables|MyBleprint|GetIsTilting)
    (Transformation|SetRelativeRotation _cube (Math|Rotator|MakeRotator (Math|Interpolation|FInterpTo _roll (Variables|MyBleprint|GetTiltAngle) _returnvalue _tiltspeed) 0.0 0.0) false false)
    (else
      (Transformation|SetRelativeRotation _cube (Math|Rotator|MakeRotator (Math|Interpolation|FInterpTo _roll 0.0 _returnvalue _tiltspeed) 0.0 0.0) false false))))

(fn ConstructionScript)